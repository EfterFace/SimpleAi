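; BPAC_Damage is an actor component that applies a stored Damage amount to its own owning actor.
; BeginPlay caches the owner, and TakeDamage subtracts Damage from the owner's BPAC_Health component if one exists.
; After each such hit it calls Dying on the owner's BPAC_Death component, if present, without checking remaining health itself.
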(event Custom|TakeDamage
  (bind _owner (Variables|Default|GetOwner))
  (bind _owner_2 (Variables|Default|GetOwner))
  (bind _returnvalue (Actor|GetComponentbyClass _owner "/Game/BluePrints/ActorComponents/BPAC_Health.BPAC_Health_C"))
  (bind _returnvalue_2 (Actor|GetComponentbyClass _owner_2 "/Game/BluePrints/ActorComponents/BPAC_Death.BPAC_Death_C"))
  (Utilities|IsValid _returnvalue
    (:Is%20Valid
      (Variables|/Game/BluePrints/ActorComponents/BPAC_Health.BPAC_Health_C|SetHealth _returnvalue (- (Variables|/Game/BluePrints/ActorComponents/BPAC_Health.BPAC_Health_C|GetHealth _returnvalue) (Variables|Default|GetDamage)))
      (Utilities|IsValid _returnvalue_2
        (:Is%20Valid
          (Default|Dying _returnvalue_2))))))

(event EventBeginPlay
  (Variables|Default|SetDamage (Variables|Default|GetDamage))
  (Variables|Default|SetOwner (Components|GetOwner)))