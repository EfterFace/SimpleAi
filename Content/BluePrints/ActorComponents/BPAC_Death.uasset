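; BPAC_Death is an actor component that handles the death of the actor it is attached to.
; It caches its owner on BeginPlay and exposes a Dying event.
; Dying looks up the owner's BPAC_Health component and, if Health is exactly zero, plays an explosion sound at the owner's location and destroys it.
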(event Custom|Dying
  (bind _owner (Variables|Default|GetOwner))
  (bind _returnvalue (Actor|GetComponentbyClass _owner "/Game/BluePrints/ActorComponents/BPAC_Health.BPAC_Health_C"))
  (Utilities|IsValid _returnvalue
    (:Is%20Valid
      (if (== (Variables|/Game/BluePrints/ActorComponents/BPAC_Health.BPAC_Health_C|GetHealth _returnvalue) 0.0)
        (Audio|PlaySoundatLocation "/Game/StarterContent/Audio/Explosion_Cue.Explosion_Cue" (Transformation|GetActorLocation (Variables|Default|GetOwner)) "0, 0, 0" 1.0 1.0 0.0 0 0 0 0)
        (Actor|DestroyActor (Variables|Default|GetOwner))))))

(event EventBeginPlay
  (Variables|Default|SetOwner (Components|GetOwner)))